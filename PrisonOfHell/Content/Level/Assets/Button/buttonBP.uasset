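; Pressure button Blueprint that reveals a hidden platform when the Dog character steps on it.
; Overlapping the sphere swaps the paper sprite to pressed, then unhides the referenced Platform and enables its collision.
; A 2D sound created at BeginPlay plays on any overlap, since it sits outside the Dog cast, and nothing reverses the press.
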(event `self.ReceiveBeginPlay`
  (bind _returnvalue (`GameplayStatics.CreateSound2D` "/Game/Sound_Design/Interactions/Button_Sound.Button_Sound" 1.0 1.0 0.0 null)))

(event `self.Sphere.OnComponentBeginOverlap`
  (params (OverlappedComponent :type "PrimitiveComponent Object Reference") (OtherActor :type "Actor Object Reference") (OtherComp :type "PrimitiveComponent Object Reference") (OtherBodyIndex :type Integer) (bFromSweep :type Boolean) (SweepResult :type "HitResult Structure (by ref)"))
  (`|ExecutionSequence`
    (:`then_0`
      (cast `/Game/Enemy/Dog/Dog` OtherActor)
      (`PaperSpriteComponent.SetSprite` (`self.PaperSprite`) "/Game/Level/Assets/Button/button_pressed_Sprite.button_pressed_Sprite")
      (`self.SetActorHiddenInGame` (`self.Platform`) false)
      (`PrimitiveComponent.SetCollisionEnabled` (`PaperGroupedSpriteActor.RenderComponent` (`self.Platform`)) "QueryAndPhysics"))
    (:`then_1`
      (`AudioComponent.Play` (stale `self.ReceiveBeginPlay` _returnvalue) 0.0))))

(fn `UserConstructionScript`)