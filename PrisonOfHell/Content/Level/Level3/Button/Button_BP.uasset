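; Level 3 pressure button that swaps which platforms are present when stepped on.
; A sphere overlap by the TestingCharacter or any of three DemonGuard classes switches the sprite to pressed.
; It then hides and disables collision on Platforms 1–2, and shows and enables collision on Platforms 3–8.
; The change is one-way, with no handling for the overlap ending.
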(event `self.Sphere.OnComponentBeginOverlap`
  (params (OverlappedComponent :type "PrimitiveComponent Object Reference") (OtherActor :type "Actor Object Reference") (OtherComp :type "PrimitiveComponent Object Reference") (OtherBodyIndex :type Integer) (bFromSweep :type Boolean) (SweepResult :type "HitResult Structure (by ref)"))
  (cast `/Game/Character/TestingCharacter` OtherActor
    (:`then`
      _)
    (:`CastFailed`
      (cast `/Game/Enemy/DemonGuard/DemonGuard1` OtherActor
        (:`then`
          _)
        (:`CastFailed`
          (cast `/Game/Enemy/DemonGuard/DemonGuard2` OtherActor
            (:`then`
              _)
            (:`CastFailed`
              (cast `/Game/Enemy/DemonGuard/DemonGuard3` OtherActor)))))))
  (`PaperSpriteComponent.SetSprite` (`self.PaperSprite`) "/Game/Level/Level3/Button/Button_Pressed_Sprite.Button_Pressed_Sprite")
  (`self.SetActorHiddenInGame` (`self.platform1`) true)
  (`PrimitiveComponent.SetCollisionEnabled` (`PaperGroupedSpriteActor.RenderComponent` (`self.platform1`)) "NoCollision")
  (`self.SetActorHiddenInGame` (`self.platform2`) true)
  (`PrimitiveComponent.SetCollisionEnabled` (`PaperGroupedSpriteActor.RenderComponent` (`self.platform2`)) "NoCollision")
  (`self.SetActorHiddenInGame` (`self.platform3`) false)
  (`PrimitiveComponent.SetCollisionEnabled` (`PaperGroupedSpriteActor.RenderComponent` (`self.platform3`)) "QueryAndPhysics")
  (`self.SetActorHiddenInGame` (`self.platform4`) false)
  (`PrimitiveComponent.SetCollisionEnabled` (`PaperGroupedSpriteActor.RenderComponent` (`self.platform4`)) "QueryAndPhysics")
  (`self.SetActorHiddenInGame` (`self.platform5`) false)
  (`PrimitiveComponent.SetCollisionEnabled` (`PaperGroupedSpriteActor.RenderComponent` (`self.platform5`)) "QueryAndPhysics")
  (`self.SetActorHiddenInGame` (`self.platform6`) false)
  (`PrimitiveComponent.SetCollisionEnabled` (`PaperGroupedSpriteActor.RenderComponent` (`self.platform6`)) "QueryAndPhysics")
  (`self.SetActorHiddenInGame` (`self.platform7`) false)
  (`PrimitiveComponent.SetCollisionEnabled` (`PaperGroupedSpriteActor.RenderComponent` (`self.platform7`)) "QueryAndPhysics")
  (`self.SetActorHiddenInGame` (`self.platform8`) false)
  (`PrimitiveComponent.SetCollisionEnabled` (`PaperGroupedSpriteActor.RenderComponent` (`self.platform8`)) "QueryAndPhysics"))

(fn `UserConstructionScript`)