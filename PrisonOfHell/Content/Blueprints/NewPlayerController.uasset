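; Player controller that switches possession between two pawn types at runtime with number keys.
; Key 1 possesses the first SoulPawn found in the level, and key 2 possesses the first TestingCharacter.
; Each press looks up actors by class and takes index zero without checking that one exists.
; BeginPlay, Tick and the construction script add no logic.
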(event `Key|One`
  (params (Key :type "Key Structure"))
  (:`Pressed`
    (bind _outactors (`GameplayStatics.GetAllActorsOfClass` "/Game/Character/SoulPawn.SoulPawn_C"))
    (`self.Possess` (`|GetArrayItem` _outactors))))

(event `Key|Two`
  (params (Key :type "Key Structure"))
  (:`Pressed`
    (bind _outactors (`GameplayStatics.GetAllActorsOfClass` "/Game/Character/TestingCharacter.TestingCharacter_C"))
    (`self.Possess` (`|GetArrayItem` _outactors))))

(fn `UserConstructionScript`
  (`parent.UserConstructionScript`))