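; Player controller for a soul-separation mechanic, swapping control between TestingCharacter, a spawned SoulPawn, and possessable guards or a dog.
; SeperateSOul spawns the soul or recalls it to the body, destroying it and releasing any possessed target.
; The possess input uses per-target FlipFlops, chosen by the soul's Near flags, with actors found via GetAllActorsOfClass.
; Tick feeds a countdown to the soul's widget and forces recall on expiry; P opens pause.
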(event `Key|P`
  (params (Key :type "Key Structure"))
  ;[1 1 1] Pause Screen
  (:`Pressed`
    (bind _returnvalue (`|CreateWidget` "/Game/Level/Widgets/Pause.Pause_C"))
    (`UserWidget.AddToViewport` _returnvalue 0)
    (set `self.bShowMouseCursor` true)
    (`GameplayStatics.SetGamePaused` true)))

(event `InputAction|SeperateSOul`
  (params (Key :type "Key Structure"))
  ;[1 1 1] seperate soul
  (:`Pressed`
    (if (`self.SoulForm?`)
      (if (`self.Possessing?`) :!label _label
        (bind _outactors (`GameplayStatics.GetAllActorsOfClass` "/Game/Character/SoulPawn.SoulPawn_C"))
        (bind _output (`|GetArrayItem` _outactors))
        (`self.DisableInput` _output null)
        (set `/Game/Character/SoulPawn.isPossessing?` false _output)
        (if (`/Game/Character/SoulPawn.NearGuard1?` _output)
          (bind _outactors_2 (`GameplayStatics.GetAllActorsOfClass` "/Game/Enemy/Guard/testingGuard.testingGuard_C"))
          (set `/Game/Enemy/Guard/testingGuard.Possesed?` false (`|GetArrayItem` _outactors_2))
          (bind _outactors_3 (`GameplayStatics.GetAllActorsOfClass` "/Game/Character/TestingCharacter.TestingCharacter_C" :!label _label_2))
          (bind _output_2 (`|GetArrayItem` _outactors_3))
          (set `/Game/Character/TestingCharacter.CurrentState` "NewEnumerator0" _output_2)
          (`self.Possess` _output_2)
          (bind _outactors_4 (`GameplayStatics.GetAllActorsOfClass` "/Game/Character/SoulPawn.SoulPawn_C"))
          (bind _output_3 (`|GetArrayItem` _outactors_4))
          (set `/Game/Character/SoulPawn.recall pressed` true _output_3)
          (set `/Game/Character/SoulPawn.SoulCounter` 0 _output_3)
          (`KismetSystemLibrary.Delay` 0.4)
          (`self.K2_DestroyActor` _output_3)
          (set `self.SoulForm?` false)
          (set `self.Duration` 20.0)
          (set `self.Possessing?` false)
          (elif (`/Game/Character/SoulPawn.NearGuard2?` _output)
            (bind _outactors_5 (`GameplayStatics.GetAllActorsOfClass` "/Game/Enemy/Guard/testingGuard1.testingGuard1_C"))
            (set `/Game/Enemy/Guard/testingGuard1.Possesed?` false (`|GetArrayItem` _outactors_5))
            (goto _label_2)
            (elif (`/Game/Character/SoulPawn.NearGuard3?` _output)
              (bind _outactors_6 (`GameplayStatics.GetAllActorsOfClass` "/Game/Enemy/Guard/testingGuard2.testingGuard2_C"))
              (set `/Game/Enemy/Guard/testingGuard2.Possesed?` false (`|GetArrayItem` _outactors_6))
              (goto _label_2)
              (elif (`/Game/Character/SoulPawn.nearDog1?` _output)
                (bind _outactors_7 (`GameplayStatics.GetAllActorsOfClass` "/Game/Enemy/Dog/Dog.Dog_C"))
                (set `/Game/Enemy/Dog/Dog.Possesed?` false (`|GetArrayItem` _outactors_7))
                (goto _label_2)))))
        (else
          (goto _label_2)))
      (else
        (bind _outactors_8 (`GameplayStatics.GetAllActorsOfClass` "/Game/Character/TestingCharacter.TestingCharacter_C"))
        (bind _output_4 (`|GetArrayItem` _outactors_8))
        (set `/Game/Character/TestingCharacter.CurrentState` "NewEnumerator4" _output_4)
        (`|SpawnActorFromClass` "/Game/Character/SoulPawn.SoulPawn_C" (`self.GetTransform` _output_4) "Undefined" "OverrideRootScale" null null)
        (bind _outactors_9 (`GameplayStatics.GetAllActorsOfClass` "/Game/Character/SoulPawn.SoulPawn_C"))
        (`self.Possess` (`|GetArrayItem` _outactors_9))
        (set `self.SoulForm?` true)))))

(event `InputAction|possess`
  (params (Key :type "Key Structure"))
  ;[1 1 1] possession mechanic
  (:`Pressed`
    (bind _outactors (`GameplayStatics.GetAllActorsOfClass` "/Game/Character/SoulPawn.SoulPawn_C"))
    (bind _output (`|GetArrayItem` _outactors))
    (if (`/Game/Character/SoulPawn.NearGuard1?` _output)
      (`/Engine/EditorBlueprintResources/StandardMacros.FlipFlop`
        (:`A`
          (set `self.Possessing?` true)
          (bind _outactors_2 (`GameplayStatics.GetAllActorsOfClass` "/Game/Character/SoulPawn.SoulPawn_C"))
          (set `/Game/Character/SoulPawn.isPossessing?` true (`|GetArrayItem` _outactors_2))
          (bind _outactors_3 (`GameplayStatics.GetAllActorsOfClass` "/Game/Enemy/Guard/testingGuard.testingGuard_C"))
          (bind _output_2 (`|GetArrayItem` _outactors_3))
          (set `/Game/Enemy/Guard/testingGuard.Possesed?` true _output_2)
          (`self.Possess` _output_2))
        (:`B`
          (set `self.Possessing?` false)
          (bind _outactors_4 (`GameplayStatics.GetAllActorsOfClass` "/Game/Character/SoulPawn.SoulPawn_C"))
          (bind _output_3 (`|GetArrayItem` _outactors_4))
          (set `/Game/Character/SoulPawn.isPossessing?` false _output_3)
          (`self.Possess` _output_3)
          (bind _outactors_5 (`GameplayStatics.GetAllActorsOfClass` "/Game/Enemy/Guard/testingGuard.testingGuard_C"))
          (set `/Game/Enemy/Guard/testingGuard.Possesed?` false (`|GetArrayItem` _outactors_5))))
      (elif (`/Game/Character/SoulPawn.NearGuard2?` _output)
        (`/Engine/EditorBlueprintResources/StandardMacros.FlipFlop`
          (:`A`
            (set `self.Possessing?` true)
            (bind _outactors_6 (`GameplayStatics.GetAllActorsOfClass` "/Game/Character/SoulPawn.SoulPawn_C"))
            (set `/Game/Character/SoulPawn.isPossessing?` true (`|GetArrayItem` _outactors_6))
            (bind _outactors_7 (`GameplayStatics.GetAllActorsOfClass` "/Game/Enemy/Guard/testingGuard1.testingGuard1_C"))
            (bind _output_4 (`|GetArrayItem` _outactors_7))
            (set `/Game/Enemy/Guard/testingGuard1.Possesed?` true _output_4)
            (`self.Possess` _output_4))
          (:`B`
            (set `self.Possessing?` false)
            (bind _outactors_8 (`GameplayStatics.GetAllActorsOfClass` "/Game/Character/SoulPawn.SoulPawn_C"))
            (bind _output_5 (`|GetArrayItem` _outactors_8))
            (set `/Game/Character/SoulPawn.isPossessing?` false _output_5)
            (`self.Possess` _output_5)
            (bind _outactors_9 (`GameplayStatics.GetAllActorsOfClass` "/Game/Enemy/Guard/testingGuard1.testingGuard1_C"))
            (set `/Game/Enemy/Guard/testingGuard1.Possesed?` false (`|GetArrayItem` _outactors_9))))
        (elif (`/Game/Character/SoulPawn.NearGuard3?` _output)
          (`/Engine/EditorBlueprintResources/StandardMacros.FlipFlop`
            (:`A`
              (set `self.Possessing?` true)
              (bind _outactors_10 (`GameplayStatics.GetAllActorsOfClass` "/Game/Character/SoulPawn.SoulPawn_C"))
              (set `/Game/Character/SoulPawn.isPossessing?` true (`|GetArrayItem` _outactors_10))
              (bind _outactors_11 (`GameplayStatics.GetAllActorsOfClass` "/Game/Enemy/Guard/testingGuard2.testingGuard2_C"))
              (bind _output_6 (`|GetArrayItem` _outactors_11))
              (set `/Game/Enemy/Guard/testingGuard2.Possesed?` true _output_6)
              (`self.Possess` _output_6))
            (:`B`
              (set `self.Possessing?` false)
              (bind _outactors_12 (`GameplayStatics.GetAllActorsOfClass` "/Game/Character/SoulPawn.SoulPawn_C"))
              (bind _output_7 (`|GetArrayItem` _outactors_12))
              (set `/Game/Character/SoulPawn.isPossessing?` false _output_7)
              (`self.Possess` _output_7)
              (bind _outactors_13 (`GameplayStatics.GetAllActorsOfClass` "/Game/Enemy/Guard/testingGuard2.testingGuard2_C"))
              (set `/Game/Enemy/Guard/testingGuard2.Possesed?` false (`|GetArrayItem` _outactors_13))))
          (elif (`/Game/Character/SoulPawn.nearDog1?` _output)
            (`/Engine/EditorBlueprintResources/StandardMacros.FlipFlop`
              (:`A`
                (set `self.Possessing?` true)
                (bind _outactors_14 (`GameplayStatics.GetAllActorsOfClass` "/Game/Character/SoulPawn.SoulPawn_C"))
                (set `/Game/Character/SoulPawn.isPossessing?` true (`|GetArrayItem` _outactors_14))
                (bind _outactors_15 (`GameplayStatics.GetAllActorsOfClass` "/Game/Enemy/Dog/Dog.Dog_C"))
                (bind _output_8 (`|GetArrayItem` _outactors_15))
                (set `/Game/Enemy/Dog/Dog.Possesed?` true _output_8)
                (`self.Possess` _output_8))
              (:`B`
                (set `self.Possessing?` false)
                (bind _outactors_16 (`GameplayStatics.GetAllActorsOfClass` "/Game/Character/SoulPawn.SoulPawn_C"))
                (bind _output_9 (`|GetArrayItem` _outactors_16))
                (set `/Game/Character/SoulPawn.isPossessing?` false _output_9)
                (`self.Possess` _output_9)
                (bind _outactors_17 (`GameplayStatics.GetAllActorsOfClass` "/Game/Enemy/Dog/Dog.Dog_C"))
                (set `/Game/Enemy/Dog/Dog.Possesed?` false (`|GetArrayItem` _outactors_17))))))))))

(event `self.ReceiveTick`
  (params (DeltaSeconds :type "Float (single-precision)"))
  (bind _duration (`self.Duration`))
  ;[1 1 1] Duration
  (if (`self.SoulForm?`)
    (if (< _duration 0.0)
      (goto _label)
      (else
        (bind _output_get (set `self.Duration` (- _duration DeltaSeconds)))
        (bind _outactors (`GameplayStatics.GetAllActorsOfClass` "/Game/Character/SoulPawn.SoulPawn_C"))
        (for _array_element _outactors
          (set `/Game/Level/Widgets/Soul_duration.Duration` _output_get (`/Game/Character/SoulPawn.TimeLeftWid` _array_element)))))))

(fn `UserConstructionScript`
  (`parent.UserConstructionScript`))